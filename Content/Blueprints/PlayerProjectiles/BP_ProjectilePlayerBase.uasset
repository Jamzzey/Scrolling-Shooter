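; Base player projectile actor that flies via a projectile movement component and damages actors it overlaps.
; The construction script applies scale and speed variables and creates a dynamic glow material, which BeginPlay tints with the projectile color.
; On overlap it applies damage, spawns a pixel explosion emitter and destroys itself.
; Otherwise, a Delay driven from Tick destroys it after a short fixed lifetime.
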(event `self.ReceiveBeginPlay`
  (`MaterialInstanceDynamic.SetVectorParameterValue` (`self.m_ProjectileMaterial`) "Color" (`self.c_ProjectileColor`)))

(event `self.ReceiveTick`
  (params (DeltaSeconds :type "Float (single-precision)"))
  (`KismetSystemLibrary.Delay` 1.2)
  (`self.K2_DestroyActor`))

(event `self.Projectile.OnComponentBeginOverlap`
  (params (OverlappedComponent :type "PrimitiveComponent Object Reference") (OtherActor :type "Actor Object Reference") (OtherComp :type "PrimitiveComponent Object Reference") (OtherBodyIndex :type Integer) (bFromSweep :type Boolean) (SweepResult :type "HitResult Structure (by ref)"))
  (`GameplayStatics.ApplyDamage` OtherActor (`self.f_Damage`))
  (`GameplayStatics.SpawnEmitterAtLocation` "/Game/Assets/Particles/P_Pixel_Explosion.P_Pixel_Explosion" (`self.K2_GetActorLocation`))
  (`self.K2_DestroyActor`))

(fn `UserConstructionScript`
  (bind _projectilemovement (`self.ProjectileMovement`))
  (bind _returnvalue (`PrimitiveComponent.CreateDynamicMaterialInstance` (`self.Projectile`) 0 "/Game/Assets/Materials/Glow/M_Glow_Projectile.M_Glow_Projectile" "None"))
  (set `self.m_ProjectileMaterial` _returnvalue)
  (`SceneComponent.SetWorldScale3D` (`self.Projectile`) (`self.v_Scale`))
  (bind _output_get (set `ProjectileMovementComponent.MaxSpeed` (`self.f_Speed`) _projectilemovement))
  (set `ProjectileMovementComponent.InitialSpeed` _output_get _projectilemovement))