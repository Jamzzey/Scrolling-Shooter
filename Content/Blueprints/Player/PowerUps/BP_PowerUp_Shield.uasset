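; BP_PowerUp_Shield is a shield power-up actor that surrounds the player and destroys projectiles that hit it.
; It caches the BP_Player pawn on BeginPlay and moves itself to the player's location every Tick rather than attaching.
; Its Sphere overlap plays a hit sound at the player and destroys any valid overlapping actor, with no class check in the graph.
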(event `self.ReceiveBeginPlay`
  ;[1 1 1] Set player references
  (bind _asbp_player (cast `/Game/Blueprints/Player/BP_Player` (`GameplayStatics.GetPlayerPawn` 0)))
  (set `self.BP_Player` _asbp_player))

(event `self.ReceiveTick`
  (params (DeltaSeconds :type "Float (single-precision)"))
  ;[1 1 1] Keeps the location same as players
  (`self.K2_SetActorLocation` (`self.K2_GetActorLocation` (`self.BP_Player`))))

(event `self.Sphere.OnComponentBeginOverlap`
  (params (OverlappedComponent :type "PrimitiveComponent Object Reference") (OtherActor :type "Actor Object Reference") (OtherComp :type "PrimitiveComponent Object Reference") (OtherBodyIndex :type Integer) (bFromSweep :type Boolean) (SweepResult :type "HitResult Structure (by ref)"))
  ;[1 1 1] Destroys projectiles on hit
  (`GameplayStatics.PlaySoundAtLocation` "/Game/Assets/Audio/ShieldHit_Clip.ShieldHit_Clip" (`self.K2_GetActorLocation` (`self.BP_Player`)) (struct) 1.0 1.0 0.0 null null null)
  (`/Engine/EditorBlueprintResources/StandardMacros.IsValid` OtherActor
    (:`Is Valid`
      (`self.K2_DestroyActor` OtherActor))))

(fn `UserConstructionScript`)