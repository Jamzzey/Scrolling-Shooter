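; BP_PickUp_AddShield is a power-up pickup that grants the player an extra shield.
; When BP_Player overlaps its static mesh, it increments that player's StartingShieldCounts and destroys itself.
; It moves upward by a fixed offset every Tick, not scaled by delta time, and self-destructs after SelfDestructTimer if not collected.
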(event `self.StaticMesh.OnComponentBeginOverlap`
  (params (OverlappedComponent :type "PrimitiveComponent Object Reference") (OtherActor :type "Actor Object Reference") (OtherComp :type "PrimitiveComponent Object Reference") (OtherBodyIndex :type Integer) (bFromSweep :type Boolean) (SweepResult :type "HitResult Structure (by ref)"))
  (bind _asbp_player (cast `/Game/Blueprints/Player/BP_Player` OtherActor))
  (set `/Game/Blueprints/Player/BP_Player.StartingShieldCounts` (+ (`/Game/Blueprints/Player/BP_Player.StartingShieldCounts` _asbp_player) 1) _asbp_player)
  (`self.K2_DestroyActor`))

(event `self.ReceiveBeginPlay`
  (`KismetSystemLibrary.Delay` (`self.SelfDestructTimer`))
  (`self.K2_DestroyActor`))

(event `self.ReceiveTick`
  (params (DeltaSeconds :type "Float (single-precision)"))
  (`self.K2_AddActorWorldOffset` (0.0 0.0 12.0)))

(fn `UserConstructionScript`)