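; BP_EnemyPath is an enemy actor that picks a random point from three location components on BeginPlay and destroys itself when its box is hit.
; A timeline is wired to lerp it between random points and fire impulse-launched BP_BulletProjectileEnemy shots behind a delay-reset flag.
; Nothing starts that timeline, so movement and shooting never run.
; Pawn sensing only casts to BP_Player, with no further action.
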(event `self.ReceiveBeginPlay`
  ;[1 1 1] creating array for locations
  (set `self.MoveToLocationPoints` (`|MakeArray` (`SceneComponent.K2_GetComponentLocation` (`self.MoveLoaction1`)) (`SceneComponent.K2_GetComponentLocation` (`self.MoveLoaction2`)) (`SceneComponent.K2_GetComponentLocation` (`self.MoveLoaction3`))))
  (`self.GetRandomLocation`))

(event `self.PawnSensing.OnSeePawn`
  (params (Pawn :type "Pawn Object Reference"))
  (cast `/Game/Blueprints/BP_Player` Pawn))

(event `self.Box.OnComponentHit`
  (params (HitComponent :type "PrimitiveComponent Object Reference") (OtherActor :type "Actor Object Reference") (OtherComp :type "PrimitiveComponent Object Reference") (NormalImpulse :type "Vector Structure") (Hit :type "HitResult Structure (by ref)"))
  ;[1 1 1] destroying
  (`self.K2_DestroyActor`))

(fn `GetLocation`
  (for (_ _array_index) (`self.MoveToLocationPoints`)
    (set `self.CurrentLocationPoint` _array_index)))

(fn `GetRandomLocation`
  (set `self.CurrentLocationPoint` (`KismetMathLibrary.RandomInteger` (`KismetArrayLibrary.Array_Length` (`self.MoveToLocationPoints`)))))

(fn `UserConstructionScript`)