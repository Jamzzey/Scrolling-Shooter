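; BP_EnemyTest is a test enemy that chases and shoots at the player once it sees them.
; PawnSensing sightings of BP_Player snap its rotation toward the player, start an AI MoveTo and attempt a shot.
; Each shot spawns BP_BulletProjectileEnemy at a spawn-location component and launches it along the Cube's forward vector with a velocity-change impulse.
; A boolean and short Delay throttle the fire rate.
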(event `self.PawnSensing.OnSeePawn`
  (params (Pawn :type "Pawn Object Reference"))
  ;[1 1 1] Enemy moving towards the player
  (bind _asbp_player (cast `/Game/Blueprints/BP_Player` Pawn))
  (`|ExecutionSequence`
    (:`then_0`
      ;[1 1 1] Rotating the enemy to face the player
      ;;[1 1 1] Enemy rotates too slow
      (`self.K2_SetActorRotation` (`KismetMathLibrary.FindLookAtRotation` (`self.K2_GetActorLocation`) (`self.K2_GetActorLocation` _asbp_player))))
    (:`then_1`
      (`|AIMoveTo` self (0.0 0.0 0.0) _asbp_player))
    (:`then_2`
      ;[1 1 1] Shooting a prjectile - A actor from a different blueprint class
      (if (`self.SpawnProjectile`)
        (bind _returnvalue (`|SpawnActorFromClass` "/Game/Blueprints/BP_BulletProjectileEnemy.BP_BulletProjectileEnemy_C" (`SceneComponent.K2_GetComponentToWorld` (`self.SpawnProjectileLoaction`)) "Undefined" "OverrideRootScale" null null))
        ;;[1 1 1 1 10] Adds impulse to enemy as well as the bullet projectile
        (`PrimitiveComponent.AddImpulse` (`/Game/Blueprints/BP_BulletProjectileEnemy.Sphere` _returnvalue) (* (`SceneComponent.GetForwardVector` (`self.Cube`)) (`self.ShootAmount`)) "None" true)
        (set `self.SpawnProjectile` false)
        (`KismetSystemLibrary.Delay` 0.2)
        (set `self.SpawnProjectile` true)))))

(fn `UserConstructionScript`)