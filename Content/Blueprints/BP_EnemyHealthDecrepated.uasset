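; An enemy actor, named as deprecated, that fires projectiles about once a second through a Delay on Tick.
; Overlapping the player damages them and destroys the enemy without drops or effects.
; Incoming damage sets FHealth from a clamped Health minus Damage; at zero it plays explosion effects, sound and camera shake, then destroys itself.
; Death can drop a pickup via nested DropChance rolls: new weapon mode, otherwise default fire rate.
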(event `self.StaticMesh.OnComponentBeginOverlap`
  (params (OverlappedComponent :type "PrimitiveComponent Object Reference") (OtherActor :type "Actor Object Reference") (OtherComp :type "PrimitiveComponent Object Reference") (OtherBodyIndex :type Integer) (bFromSweep :type Boolean) (SweepResult :type "HitResult Structure (by ref)"))
  ;[1 1 1] Collision with Player, set to destroy the enemy for now
  (bind _asbp_player (cast `/Game/Blueprints/BP_Player` OtherActor))
  (`KismetSystemLibrary.PrintString` "Player has been damaged!" true true (struct :`G` 0.66 :`B` 1.0 :`A` 1.0) 5.0)
  (`GameplayStatics.ApplyDamage` _asbp_player (`self.Damage`))
  (`self.K2_DestroyActor`))

(event `self.ReceiveAnyDamage`
  (params (Damage :type "Float (single-precision)") (DamageType :type "DamageType Object Reference") (InstigatedBy :type "Controller Object Reference") (DamageCauser :type "Actor Object Reference"))
  (bind _returnvalue (`self.K2_GetActorLocation`))
  (bind _returnvalue_2 (`self.GetTransform`))
  ;[1 1 1] Health Calculation
  (set `self.f_Health` (`KismetMathLibrary.FClamp` (- (`self.Health`) Damage) 0.0 (`self.Max Health`)))
  (if (<= (`self.f_Health`) 0.0)
    (if (< (`KismetMathLibrary.RandomFloat`) (`self.Drop Chance`))
      (if (< (`KismetMathLibrary.RandomFloat`) (`self.Drop Chance`))
        ;[1 1 1] Set the Power Ups here
        (`|SpawnActorFromClass` "/Game/Blueprints/WeaponCollectible/BP_PickUp_NewWeaponMode.BP_PickUp_NewWeaponMode_C" _returnvalue_2 "Undefined" "OverrideRootScale" null null)
        (elif (< (`KismetMathLibrary.RandomFloat`) (`self.Drop Chance`))
          (`|SpawnActorFromClass` "/Game/Blueprints/PickUps/BP_PickUp_DefaultFireRate.BP_PickUp_DefaultFireRate_C" _returnvalue_2 "Undefined" "OverrideRootScale" null null)
          (else
            (`|SpawnActorFromClass` "/Game/Blueprints/PickUps/BP_PickUp_DefaultFireRate.BP_PickUp_DefaultFireRate_C" _returnvalue_2 "Undefined" "OverrideRootScale" null null)))))
    ;[1 1 1] Player Feedback, FX, Shake and Sound
    (`GameplayStatics.SpawnEmitterAtLocation` "/Game/Assets/Particles/P_Pixel_Explosion_Player.P_Pixel_Explosion_Player" _returnvalue)
    (`GameplayStatics.PlayWorldCameraShake` "/Game/Blueprints/BP_CameraShake.BP_CameraShake_C" _returnvalue 0.0 500.0)
    (`GameplayStatics.PlaySoundAtLocation` "/Game/Assets/Audio/Explosion.Explosion" _returnvalue (struct) 1.0 1.0 0.0 null null null)
    (`KismetSystemLibrary.PrintString` "Enemy is dead!")
    (`self.K2_DestroyActor`)))

(event `self.ReceiveTick`
  (params (DeltaSeconds :type "Float (single-precision)"))
  (`KismetSystemLibrary.Delay` 1.0)
  (`self.EnemyDefaultFire` (`SceneComponent.K2_GetComponentToWorld` (`self.Shooting direction`))))

(fn `EnemyDefaultFire`
  (params (Spawn :type "Transform Structure"))
  (`|SpawnActorFromClass` "/Game/Blueprints/EnemyProjectiles/BP_ProjectileEnemyDefault.BP_ProjectileEnemyDefault_C" Spawn "AlwaysSpawn" "OverrideRootScale" null (`self.Projectile Color`) self))

(fn `UserConstructionScript`)