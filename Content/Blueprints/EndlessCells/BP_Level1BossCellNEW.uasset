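; Level 1 boss cell for the endless-cell level, which sets up the BP_Boss1 encounter.
; BeginPlay runs the parent logic, then spawns the boss at SpawnEnemy and adds the enemy HP widget to the viewport.
; Ending overlap with SpawnTrigger spawns a widened BP_BossGate at Scene1, while filter volumes destroy actors that begin overlapping them.
; Tick is empty; the DeleteEnemies sweep of enemies and spawners is disconnected and never runs.
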(event `self.ReceiveBeginPlay`
  ;[1 1 1] Spawns boss and creates HUD
  (`parent.ReceiveBeginPlay`)
  (`/Engine/EditorBlueprintResources/StandardMacros.DoOnce` false
    (:`Completed`
      (`|SpawnActorFromClass` "/Game/Blueprints/EnemyAI/BP_Boss1.BP_Boss1_C" (`SceneComponent.K2_GetComponentToWorld` (`self.SpawnEnemy`)) "Undefined" "OverrideRootScale" null null)
      (bind _returnvalue (`|CreateWidget` "/Game/Blueprints/GUI/BPW_EnemyHP.BPW_EnemyHP_C"))
      (bind _output_get (set `self.BPW_EnemyHP` _returnvalue))
      (`UserWidget.AddToViewport` _output_get 0))))

(event `self.ReceiveTick`
  (params (DeltaSeconds :type "Float (single-precision)"))
  ;[1 1 1] Cleans up all enemies
)

(event `self.SpawnTrigger.OnComponentEndOverlap`
  (params (OverlappedComponent :type "PrimitiveComponent Object Reference") (OtherActor :type "Actor Object Reference") (OtherComp :type "PrimitiveComponent Object Reference") (OtherBodyIndex :type Integer))
  (`|SpawnActorFromClass` "/Game/Blueprints/EndlessCells/BP_BossGate.BP_BossGate_C" (`KismetMathLibrary.MakeTransform` (`SceneComponent.K2_GetComponentLocation` (`self.Scene1`)) (struct) (5.0 1.0 1.0)) "Undefined" "OverrideRootScale" null null))

(event `self.enemyfilter.OnComponentBeginOverlap`
  (params (OverlappedComponent :type "PrimitiveComponent Object Reference") (OtherActor :type "Actor Object Reference") (OtherComp :type "PrimitiveComponent Object Reference") (OtherBodyIndex :type Integer) (bFromSweep :type Boolean) (SweepResult :type "HitResult Structure (by ref)"))
  (`/Engine/EditorBlueprintResources/StandardMacros.IsValid` OtherActor
    (:`Is Valid`
      (`self.K2_DestroyActor` OtherActor))))

(event `self.spawnerfilters.OnComponentBeginOverlap`
  (params (OverlappedComponent :type "PrimitiveComponent Object Reference") (OtherActor :type "Actor Object Reference") (OtherComp :type "PrimitiveComponent Object Reference") (OtherBodyIndex :type Integer) (bFromSweep :type Boolean) (SweepResult :type "HitResult Structure (by ref)"))
  (`self.K2_DestroyActor` OtherActor))

(event `self.spawnerfilters1.OnComponentBeginOverlap`
  (params (OverlappedComponent :type "PrimitiveComponent Object Reference") (OtherActor :type "Actor Object Reference") (OtherComp :type "PrimitiveComponent Object Reference") (OtherBodyIndex :type Integer) (bFromSweep :type Boolean) (SweepResult :type "HitResult Structure (by ref)"))
  (`self.K2_DestroyActor` OtherActor))

(fn `UserConstructionScript`
  (`parent.UserConstructionScript`))