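; BP_SpawnerCellHard is a cell actor for the endless cells level that places enemy spawners and exposes an Attachpoint transform.
; Any actor or component ending overlap with SpawnTrigger spawns an EnemySpawner at each of two spawn locations, with no player check.
; The player entering EndTrigger destroys the cell after five seconds; leaving it calls AddSpawner on BP_GameMode.
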(event `self.EndTrigger.OnComponentEndOverlap`
  (params (OverlappedComponent :type "PrimitiveComponent Object Reference") (OtherActor :type "Actor Object Reference") (OtherComp :type "PrimitiveComponent Object Reference") (OtherBodyIndex :type Integer))
  (if (== OtherActor (`GameplayStatics.GetPlayerPawn` 0))
    (bind _asbp_game_mode (cast `/Game/Blueprints/GeneralGameBP/BP_GameMode` (`GameplayStatics.GetGameMode`)))
    (`/Game/Blueprints/GeneralGameBP/BP_GameMode.AddSpawner` _asbp_game_mode)))

(event `self.EndTrigger.OnComponentBeginOverlap`
  (params (OverlappedComponent :type "PrimitiveComponent Object Reference") (OtherActor :type "Actor Object Reference") (OtherComp :type "PrimitiveComponent Object Reference") (OtherBodyIndex :type Integer) (bFromSweep :type Boolean) (SweepResult :type "HitResult Structure (by ref)"))
  (if (== OtherActor (`GameplayStatics.GetPlayerPawn` 0))
    (`KismetSystemLibrary.Delay` 5.0)
    (`self.K2_DestroyActor`)))

(event `self.SpawnTrigger.OnComponentEndOverlap`
  (params (OverlappedComponent :type "PrimitiveComponent Object Reference") (OtherActor :type "Actor Object Reference") (OtherComp :type "PrimitiveComponent Object Reference") (OtherBodyIndex :type Integer))
  (`|SpawnActorFromClass` (`self.EnemySpawner`) (`SceneComponent.K2_GetComponentToWorld` (`self.SpawnLocation1`)) "Undefined" "OverrideRootScale" null null)
  (`|SpawnActorFromClass` (`self.EnemySpawner`) (`SceneComponent.K2_GetComponentToWorld` (`self.SpawnLocation2`)) "Undefined" "OverrideRootScale" null null))

(fn `GetAttachpointTransform`
  (returns (Attachtransform :type "Transform Structure"))
  (return (`SceneComponent.K2_GetComponentToWorld` (`self.Attachpoint`))))

(fn `UserConstructionScript`)