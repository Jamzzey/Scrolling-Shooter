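; BP_BossTrigger is a trigger actor for the boss encounter, with two overlap volumes.
; Overlapping EndTrigger sets BossSpawned to false on the game mode, which the graph notes is for an early camera switch.
; EnemyFilter destroys any actor that overlaps it, with no class check.
; An unconnected, unused branch holds an alternate BP_Boss1 spawn at SpawnEnemy with an enemy HP widget.
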(event `self.EndTrigger.OnComponentBeginOverlap`
  (params (OverlappedComponent :type "PrimitiveComponent Object Reference") (OtherActor :type "Actor Object Reference") (OtherComp :type "PrimitiveComponent Object Reference") (OtherBodyIndex :type Integer) (bFromSweep :type Boolean) (SweepResult :type "HitResult Structure (by ref)"))
  ;[1 1 1] Sets boss spawned early to have camera switch
  (set `/Game/Blueprints/BP_GameMode.BossSpawned` false (`self.BP_GameMode`)))

(event `self.EnemyFilter.OnComponentBeginOverlap`
  (params (OverlappedComponent :type "PrimitiveComponent Object Reference") (OtherActor :type "Actor Object Reference") (OtherComp :type "PrimitiveComponent Object Reference") (OtherBodyIndex :type Integer) (bFromSweep :type Boolean) (SweepResult :type "HitResult Structure (by ref)"))
  ;[1 1 1] Enemy filter
  (`self.K2_DestroyActor` OtherActor))

(fn `UserConstructionScript`
  (`parent.UserConstructionScript`))