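; BP_SpawnerCellNormal is an endless-level cell that spawns enemy spawners and destroys itself once traversed.
; When any actor leaves SpawnTrigger, it spawns two EnemySpawner actors at fixed locations unless the game mode reports a spawned boss.
; The player entering EndTrigger starts a five-second destroy delay, and leaving it calls AddSpawner on BP_GameMode.
; GetAttachpointTransform exposes the cell's attach point transform.
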(event `self.ReceiveBeginPlay`
  (bind _asbp_game_mode (cast `/Game/Blueprints/BP_GameMode` (`GameplayStatics.GetGameMode`)))
  (set `self.BP_GameMode` _asbp_game_mode))

(event `self.EndTrigger.OnComponentEndOverlap`
  (params (OverlappedComponent :type "PrimitiveComponent Object Reference") (OtherActor :type "Actor Object Reference") (OtherComp :type "PrimitiveComponent Object Reference") (OtherBodyIndex :type Integer))
  (if (== OtherActor (`GameplayStatics.GetPlayerPawn` 0))
    (`/Game/Blueprints/BP_GameMode.AddSpawner` (`self.BP_GameMode`))))

(event `self.SpawnTrigger.OnComponentEndOverlap`
  (params (OverlappedComponent :type "PrimitiveComponent Object Reference") (OtherActor :type "Actor Object Reference") (OtherComp :type "PrimitiveComponent Object Reference") (OtherBodyIndex :type Integer))
  (if (not (`/Game/Blueprints/BP_GameMode.BossSpawned` (`self.BP_GameMode`)))
    (`|SpawnActorFromClass` (`self.EnemySpawner`) (`SceneComponent.K2_GetComponentToWorld` (`self.SpawnLocation1`)) "Undefined" "OverrideRootScale" null null)
    (`|SpawnActorFromClass` (`self.EnemySpawner`) (`SceneComponent.K2_GetComponentToWorld` (`self.SpawnLocation2`)) "Undefined" "OverrideRootScale" null null)))

(event `self.EndTrigger.OnComponentBeginOverlap`
  (params (OverlappedComponent :type "PrimitiveComponent Object Reference") (OtherActor :type "Actor Object Reference") (OtherComp :type "PrimitiveComponent Object Reference") (OtherBodyIndex :type Integer) (bFromSweep :type Boolean) (SweepResult :type "HitResult Structure (by ref)"))
  (if (== OtherActor (`GameplayStatics.GetPlayerPawn` 0))
    (`KismetSystemLibrary.Delay` 5.0)
    (`self.K2_DestroyActor`)))

(fn `GetAttachpointTransform`
  (returns (Attachtransform :type "Transform Structure"))
  (return (`SceneComponent.K2_GetComponentToWorld` (`self.Attachpoint`))))

(fn `UserConstructionScript`)