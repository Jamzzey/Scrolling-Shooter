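; BP_ObstaclePosition3 is an obstacle segment for an endless level, exposing attach-point and billboard transforms.
; When the player leaves EndTrigger, it asks BP_GameMode to add another obstacle; entering that trigger starts a delayed self-destruct.
; Hitting the Cube triggers the player's collision camera shake, applies environmental damage and destroys the whole actor.
; Its AnyDamage handler reduces clamped health and destroys the actor at zero.
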(event `self.EndTrigger.OnComponentEndOverlap`
  (params (OverlappedComponent :type "PrimitiveComponent Object Reference") (OtherActor :type "Actor Object Reference") (OtherComp :type "PrimitiveComponent Object Reference") (OtherBodyIndex :type Integer))
  (if (== OtherActor (`GameplayStatics.GetPlayerPawn` 0))
    (bind _asbp_game_mode (cast `/Game/Blueprints/BP_GameMode` (`GameplayStatics.GetGameMode`)))
    (`/Game/Blueprints/BP_GameMode.AddObstacle` _asbp_game_mode)))

(event `self.EndTrigger.OnComponentBeginOverlap`
  (params (OverlappedComponent :type "PrimitiveComponent Object Reference") (OtherActor :type "Actor Object Reference") (OtherComp :type "PrimitiveComponent Object Reference") (OtherBodyIndex :type Integer) (bFromSweep :type Boolean) (SweepResult :type "HitResult Structure (by ref)"))
  (if (== OtherActor (`GameplayStatics.GetPlayerPawn` 0))
    (`KismetSystemLibrary.Delay` 5.0)
    (`self.K2_DestroyActor`)))

(event `self.Cube.OnComponentBeginOverlap`
  (params (OverlappedComponent :type "PrimitiveComponent Object Reference") (OtherActor :type "Actor Object Reference") (OtherComp :type "PrimitiveComponent Object Reference") (OtherBodyIndex :type Integer) (bFromSweep :type Boolean) (SweepResult :type "HitResult Structure (by ref)"))
  (bind _asbp_player (cast `/Game/Blueprints/BP_Player` OtherActor))
  (`/Game/Blueprints/BP_Player.CameraShakeCollision` _asbp_player)
  (`GameplayStatics.ApplyDamage` null (`self.Environmental Damage`))
  (`self.K2_DestroyActor`))

(event `self.ReceiveAnyDamage`
  (params (Damage :type "Float (single-precision)") (DamageType :type "DamageType Object Reference") (InstigatedBy :type "Controller Object Reference") (DamageCauser :type "Actor Object Reference"))
  (set `self.f_Health` (`KismetMathLibrary.FClamp` (- (`self.f_Health`) Damage) 0.0 (`self.f_MaxHealth`)))
  (if (<= (`self.f_Health`) 0.0)
    (`self.K2_DestroyActor`)))

(fn `GetAttachpointTransform`
  (returns (Attachtransform :type "Transform Structure"))
  (return (`SceneComponent.K2_GetComponentToWorld` (`self.Attachpoint`))))

(fn `GetBillboardTransform`
  (returns (Spawn :type "Transform Structure"))
  (return (`SceneComponent.K2_GetComponentToWorld` (`self.BillboardAttach`))))

(fn `UserConstructionScript`)