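; BP_CellOne is a level cell for an endless-cell system that may place an enemy spawner at BeginPlay, based on SpawnChance.
; When the player leaves EndTrigger, it asks BP_GameMode for a normal, medium, hard or boss cell by CellSpawned count, zeroing player vertical speed for the boss.
; Entering EndTrigger destroys the cell after a delay, and BulletFilter destroys overlapping actors.
; GetAttachpointTransform exposes the Attachpoint transform.
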(event `self.ReceiveBeginPlay`
  (bind _asbp_game_mode (cast `/Game/Blueprints/BP_GameMode` (`GameplayStatics.GetGameMode`)))
  (set `self.BP_GameMode` _asbp_game_mode)
  (bind _asbp_player (cast `/Game/Blueprints/BP_Player` (`GameplayStatics.GetPlayerPawn` 0)))
  (set `self.BP_Player` _asbp_player)
  (if (< (`KismetMathLibrary.RandomFloat`) (`self.SpawnChance`))
    (`|SpawnActorFromClass` "/Game/Blueprints/EnemyAI/BP_EnemySpawner.BP_EnemySpawner_C" (`SceneComponent.K2_GetComponentToWorld` (`self.SpawnEnemy`)) "Undefined" "OverrideRootScale" null null)))

(event `self.EndTrigger.OnComponentEndOverlap`
  (params (OverlappedComponent :type "PrimitiveComponent Object Reference") (OtherActor :type "Actor Object Reference") (OtherComp :type "PrimitiveComponent Object Reference") (OtherBodyIndex :type Integer))
  (bind _bp_gamemode (`self.BP_GameMode`))
  (bind _cellspawned (`/Game/Blueprints/BP_GameMode.CellSpawned` (`self.BP_GameMode`)))
  (if (== OtherActor (`GameplayStatics.GetPlayerPawn` 0))
    (bind _asbp_game_mode (cast `/Game/Blueprints/BP_GameMode` (`GameplayStatics.GetGameMode`)))
    (if (< _cellspawned 3)
      (`/Game/Blueprints/BP_GameMode.AddCell` _asbp_game_mode)
      (`KismetSystemLibrary.PrintString` "Normal Cell is spawning")
      (elif (< _cellspawned 6)
        (`/Game/Blueprints/BP_GameMode.AddMediumCell` _asbp_game_mode)
        (`KismetSystemLibrary.PrintString` "Medium Cells are spawning")
        (elif (< _cellspawned 12)
          (`/Game/Blueprints/BP_GameMode.AddHardCell` _asbp_game_mode)
          (`KismetSystemLibrary.PrintString` "Spawning Hard")
          (else
            (set `/Game/Blueprints/BP_Player.f_VerticalSpeed` 0.0 (`self.BP_Player`))
            (`/Game/Blueprints/BP_GameMode.AddBossCell` _asbp_game_mode)
            (`KismetSystemLibrary.PrintString` "Boss is spawning")))))
    (bind _output_get (set `/Game/Blueprints/BP_GameMode.CellSpawned` (+ (`/Game/Blueprints/BP_GameMode.CellSpawned` _bp_gamemode) 1) _bp_gamemode))
    (`KismetSystemLibrary.PrintString` (`KismetStringLibrary.Conv_IntToString` _output_get))))

(event `self.EndTrigger.OnComponentBeginOverlap`
  (params (OverlappedComponent :type "PrimitiveComponent Object Reference") (OtherActor :type "Actor Object Reference") (OtherComp :type "PrimitiveComponent Object Reference") (OtherBodyIndex :type Integer) (bFromSweep :type Boolean) (SweepResult :type "HitResult Structure (by ref)"))
  (if (== OtherActor (`GameplayStatics.GetPlayerPawn` 0))
    (`KismetSystemLibrary.Delay` 2.0)
    (`self.K2_DestroyActor`)))

(event `self.bulletFilter.OnComponentBeginOverlap`
  (params (OverlappedComponent :type "PrimitiveComponent Object Reference") (OtherActor :type "Actor Object Reference") (OtherComp :type "PrimitiveComponent Object Reference") (OtherBodyIndex :type Integer) (bFromSweep :type Boolean) (SweepResult :type "HitResult Structure (by ref)"))
  (`self.K2_DestroyActor` OtherActor))

(fn `GetAttachpointTransform`
  (returns (Attachtransform :type "Transform Structure"))
  (return (`SceneComponent.K2_GetComponentToWorld` (`self.Attachpoint`))))

(fn `UserConstructionScript`)