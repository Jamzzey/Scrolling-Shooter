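; Base level segment for the endless cell system, which chains cells as the player moves through them.
; Leaving EndTrigger asks BP_GameMode for the next cell, escalating from normal through medium, hard and pre-boss by spawn count, then stops player movement for the boss cell.
; Entering EndTrigger starts the cell's delayed self-destruction.
; SpawnTrigger exits create two enemy spawners, and BulletFilter destroys any actor entering it.
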(event `self.ReceiveBeginPlay`
  ;[1 1 1] Get variables
  (bind _asbp_game_mode (cast `/Game/Blueprints/BP_GameMode` (`GameplayStatics.GetGameMode`)))
  (set `self.BP_GameMode` _asbp_game_mode)
  (bind _asbp_player (cast `/Game/Blueprints/BP_Player` (`GameplayStatics.GetPlayerPawn` 0)))
  (set `self.BP_Player` _asbp_player))

(event `self.EndTrigger.OnComponentEndOverlap`
  (params (OverlappedComponent :type "PrimitiveComponent Object Reference") (OtherActor :type "Actor Object Reference") (OtherComp :type "PrimitiveComponent Object Reference") (OtherBodyIndex :type Integer))
  (bind _bp_gamemode (`self.BP_GameMode`))
  (if (== OtherActor (`GameplayStatics.GetPlayerPawn` 0))
    (if (not (`/Game/Blueprints/BP_GameMode.BossSpawned` (`self.BP_GameMode`)))
      (bind _asbp_game_mode (cast `/Game/Blueprints/BP_GameMode` (`GameplayStatics.GetGameMode`)))
      (if (< (`/Game/Blueprints/BP_GameMode.CellSpawned` (`self.BP_GameMode`)) 2)
        (`/Game/Blueprints/BP_GameMode.AddNormalCell` _asbp_game_mode)
        (set `/Game/Blueprints/BP_GameMode.CellSpawned` (+ (`/Game/Blueprints/BP_GameMode.CellSpawned` _bp_gamemode) 1) _bp_gamemode :!label _label)
        (elif (< (`/Game/Blueprints/BP_GameMode.CellSpawned` (`self.BP_GameMode`)) 4)
          (`/Game/Blueprints/BP_GameMode.AddMediumCell` _asbp_game_mode)
          (goto _label)
          (elif (< (`/Game/Blueprints/BP_GameMode.CellSpawned` (`self.BP_GameMode`)) 6)
            (`/Game/Blueprints/BP_GameMode.AddHardCell` _asbp_game_mode)
            (goto _label)
            (elif (< (`/Game/Blueprints/BP_GameMode.CellSpawned` (`self.BP_GameMode`)) 7)
              (`/Game/Blueprints/BP_GameMode.AddPreBossCell` _asbp_game_mode)
              (goto _label)
              (elif (`/Game/Blueprints/BP_GameMode.LevelOneBossDead` (`self.BP_GameMode`))
                (set `/Game/Blueprints/BP_Player.b_StopMovement` true (`self.BP_Player`))
                (`/Game/Blueprints/BP_GameMode.AddBossCell` _asbp_game_mode)
                (set `/Game/Blueprints/BP_GameMode.BossSpawned` true (`self.BP_GameMode`))
                (else
                  (set `/Game/Blueprints/BP_Player.b_StopMovement` true (`self.BP_Player`))
                  (`/Game/Blueprints/BP_GameMode.AddBossCell` _asbp_game_mode)
                  (set `/Game/Blueprints/BP_GameMode.BossSpawned` true (`self.BP_GameMode`))
                  (goto _label))))))))))

(event `self.EndTrigger.OnComponentBeginOverlap`
  (params (OverlappedComponent :type "PrimitiveComponent Object Reference") (OtherActor :type "Actor Object Reference") (OtherComp :type "PrimitiveComponent Object Reference") (OtherBodyIndex :type Integer) (bFromSweep :type Boolean) (SweepResult :type "HitResult Structure (by ref)"))
  (if (== OtherActor (`GameplayStatics.GetPlayerPawn` 0))
    (`KismetSystemLibrary.Delay` (`self.SelfDestroyTimer`))
    (`self.K2_DestroyActor`)))

(event `self.bulletFilter.OnComponentBeginOverlap`
  (params (OverlappedComponent :type "PrimitiveComponent Object Reference") (OtherActor :type "Actor Object Reference") (OtherComp :type "PrimitiveComponent Object Reference") (OtherBodyIndex :type Integer) (bFromSweep :type Boolean) (SweepResult :type "HitResult Structure (by ref)"))
  (`self.K2_DestroyActor` OtherActor))

(event `self.SpawnTrigger.OnComponentEndOverlap`
  (params (OverlappedComponent :type "PrimitiveComponent Object Reference") (OtherActor :type "Actor Object Reference") (OtherComp :type "PrimitiveComponent Object Reference") (OtherBodyIndex :type Integer))
  (`|SpawnActorFromClass` (`self.EnemySpawner`) (`SceneComponent.K2_GetComponentToWorld` (`self.SpawnEnemy`)) "Undefined" "OverrideRootScale" null null)
  (`|SpawnActorFromClass` (`self.EnemySpawner`) (`SceneComponent.K2_GetComponentToWorld` (`self.SpawnEnemy1`)) "Undefined" "OverrideRootScale" null null))

(fn `GetAttachpointTransform`
  (returns (Attachtransform :type "Transform Structure"))
  (return (`SceneComponent.K2_GetComponentToWorld` (`self.Attachpoint`))))

(fn `UserConstructionScript`)