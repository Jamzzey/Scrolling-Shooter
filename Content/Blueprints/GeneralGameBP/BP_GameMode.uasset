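; Game mode that builds the level from chained cells and tracks score, multiplier and enemy kills.
; BeginPlay spawns random normal cells, obstacles and CellSpawned-tiered spawners, each advancing NextSpawnPoint to its attach point; harder-cell and boss helpers also exist.
; GameOver shows its widget and saves the high score to a save slot.
; HUD, music and score-loading setup is disconnected, and LoadScore and SaveScore are empty.
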(event `self.ReceiveBeginPlay`
  ;[1 1 1] Set up HUD and Score Systems
  ;[1 1 1] Spawn Level
  (for _ (range 2)
    (`self.AddNormalCell`)
    (`self.AddObstacle`)
    (`self.AddSpawner`)))

(event `self.ReceiveTick`
  (params (DeltaSeconds :type "Float (single-precision)"))
  ;[1 1 1] Score Hierarchy
  ;;[1 1 1] Resets Multiplier after a while
  (if (>= (`self.i_Multiplier`) 0)
    (`KismetSystemLibrary.Delay` 2.0)
    (set `self.i_Multiplier` (- (`self.i_Multiplier`) 1))
    (else
      (set `self.i_Multiplier` 0))))

(event `self.ReceiveEndPlay`
  (params (EndPlayReason :type "EEndPlayReason Enum" :default "Destroyed"))
  ;[1 1 1] Score Hierarchy
  ;;[1 1 1] Saves the Score
  (`self.SaveScore`))

(event `Multiply`
  ;[1 1 1] Score Hierarchy
  ;;[1 1 1] Score Multiplier
  (bind _outactors (`GameplayStatics.GetAllActorsOfClass` "/Game/Blueprints/EnemyAI/BP_EnemyBase.BP_EnemyBase_C"))
  (set `self.BP_EnemyBase` _outactors)
  (set `self.i_Score` (* (`self.i_Score`) (`self.i_Multiplier`))))

(event `CheckEnemyCount`
  (params (Value :type Integer)))

(fn `AddBoss1Cell`
  (`/Engine/EditorBlueprintResources/StandardMacros.DoOnce` false
    (:`Completed`
      (`|SpawnActorFromClass` "/Game/Blueprints/EndlessCells/BP_Level1BossCell.BP_Level1BossCell_C" (`self.NextSpawnPoint`) "Undefined" "OverrideRootScale" null null))))

(fn `AddBoss2Cell`
  (`/Engine/EditorBlueprintResources/StandardMacros.DoOnce` false
    (:`Completed`
      (`|MultiGate` true
        (:`Out 0`
          (`|SpawnActorFromClass` "/Game/Blueprints/EndlessCells/BP_Level2BossCell.BP_Level2BossCell_C" (`self.NextSpawnPoint`) "Undefined" "OverrideRootScale" null null))
        (:`Out 1`
          (`|SpawnActorFromClass` "/Game/Blueprints/EndlessCells/BP_Level2BossCell.BP_Level2BossCell_C" (`self.NextSpawnPoint`) "Undefined" "OverrideRootScale" null null))
        (:`Out 2`
          (`|SpawnActorFromClass` "/Game/Blueprints/EndlessCells/BP_Level2BossCell.BP_Level2BossCell_C" (`self.NextSpawnPoint`) "Undefined" "OverrideRootScale" null null))))))

(fn `AddBossTriggerCell`
  (`/Engine/EditorBlueprintResources/StandardMacros.DoOnce` false
    (:`Completed`
      (bind _returnvalue (`|SpawnActorFromClass` "/Game/Blueprints/EndlessCells/BP_BossTrigger.BP_BossTrigger_C" (`self.NextSpawnPoint`) "Undefined" "OverrideRootScale" null null))
      (bind _attachtransform (`/Game/Blueprints/EndlessCells/BP_BaseCell.GetAttachpointTransform` _returnvalue))
      (set `self.NextSpawnPoint` _attachtransform))))

(fn `AddHardCell`
  (`|MultiGate` true
    (:`Out 0`
      (bind _returnvalue (`|SpawnActorFromClass` "/Game/Blueprints/EndlessCells/BP_HardCell1.BP_HardCell1_C" (`self.NextSpawnPoint`) "Undefined" "OverrideRootScale" null null))
      (bind _attachtransform (`/Game/Blueprints/EndlessCells/BP_BaseCell.GetAttachpointTransform` _returnvalue))
      (set `self.NextSpawnPoint` _attachtransform))
    (:`Out 1`
      (bind _returnvalue_2 (`|SpawnActorFromClass` "/Game/Blueprints/EndlessCells/BP_HardCell2.BP_HardCell2_C" (`self.NextSpawnPoint`) "Undefined" "OverrideRootScale" null null))
      (bind _attachtransform_2 (`/Game/Blueprints/EndlessCells/BP_BaseCell.GetAttachpointTransform` _returnvalue_2))
      (set `self.NextSpawnPoint` _attachtransform_2))
    (:`Out 2`
      (bind _returnvalue_3 (`|SpawnActorFromClass` "/Game/Blueprints/EndlessCells/BP_HardCell3.BP_HardCell3_C" (`self.NextSpawnPoint`) "Undefined" "OverrideRootScale" null null))
      (bind _attachtransform_3 (`/Game/Blueprints/EndlessCells/BP_BaseCell.GetAttachpointTransform` _returnvalue_3))
      (set `self.NextSpawnPoint` _attachtransform_3))))

(fn `AddMediumCell`
  (`|MultiGate` true
    (:`Out 0`
      (bind _returnvalue (`|SpawnActorFromClass` "/Game/Blueprints/EndlessCells/BP_MediumCell1.BP_MediumCell1_C" (`self.NextSpawnPoint`) "Undefined" "OverrideRootScale" null null))
      (bind _attachtransform (`/Game/Blueprints/EndlessCells/BP_BaseCell.GetAttachpointTransform` _returnvalue))
      (set `self.NextSpawnPoint` _attachtransform))
    (:`Out 1`
      (bind _returnvalue_2 (`|SpawnActorFromClass` "/Game/Blueprints/EndlessCells/BP_MediumCell2.BP_MediumCell2_C" (`self.NextSpawnPoint`) "Undefined" "OverrideRootScale" null null))
      (bind _attachtransform_2 (`/Game/Blueprints/EndlessCells/BP_BaseCell.GetAttachpointTransform` _returnvalue_2))
      (set `self.NextSpawnPoint` _attachtransform_2))
    (:`Out 2`
      (bind _returnvalue_3 (`|SpawnActorFromClass` "/Game/Blueprints/EndlessCells/BP_MediumCell3.BP_MediumCell3_C" (`self.NextSpawnPoint`) "Undefined" "OverrideRootScale" null null))
      (bind _attachtransform_3 (`/Game/Blueprints/EndlessCells/BP_BaseCell.GetAttachpointTransform` _returnvalue_3))
      (set `self.NextSpawnPoint` _attachtransform_3))))

(fn `AddNormalCell`
  (`|MultiGate` true
    (:`Out 0`
      (bind _returnvalue (`|SpawnActorFromClass` "/Game/Blueprints/EndlessCells/BP_NormalCell1.BP_NormalCell1_C" (`self.NextSpawnPoint`) "Undefined" "OverrideRootScale" null null))
      (bind _attachtransform (`/Game/Blueprints/EndlessCells/BP_BaseCell.GetAttachpointTransform` _returnvalue))
      (set `self.NextSpawnPoint` _attachtransform))
    (:`Out 1`
      (bind _returnvalue_2 (`|SpawnActorFromClass` "/Game/Blueprints/EndlessCells/BP_NormalCell2.BP_NormalCell2_C" (`self.NextSpawnPoint`) "Undefined" "OverrideRootScale" null null))
      (bind _attachtransform_2 (`/Game/Blueprints/EndlessCells/BP_BaseCell.GetAttachpointTransform` _returnvalue_2))
      (set `self.NextSpawnPoint` _attachtransform_2))
    (:`Out 2`
      (bind _returnvalue_3 (`|SpawnActorFromClass` "/Game/Blueprints/EndlessCells/BP_NormalCell3.BP_NormalCell3_C" (`self.NextSpawnPoint`) "Undefined" "OverrideRootScale" null null))
      (bind _attachtransform_3 (`/Game/Blueprints/EndlessCells/BP_BaseCell.GetAttachpointTransform` _returnvalue_3))
      (set `self.NextSpawnPoint` _attachtransform_3))))

(fn `AddObstacle`
  (`|MultiGate` true
    (:`Out 0`
      (bind _returnvalue (`|SpawnActorFromClass` "/Game/Blueprints/EndlessCells/BP_ObstaclePosition1.BP_ObstaclePosition1_C" (`self.NextSpawnPoint`) "Undefined" "OverrideRootScale" null null))
      (bind _attachtransform (`/Game/Blueprints/EndlessCells/BP_ObstaclePosition1.GetAttachpointTransform` _returnvalue))
      (set `self.NextSpawnPoint` _attachtransform))
    (:`Out 1`
      (bind _returnvalue_2 (`|SpawnActorFromClass` "/Game/Blueprints/EndlessCells/BP_ObstaclePosition2.BP_ObstaclePosition2_C" (`self.NextSpawnPoint`) "Undefined" "OverrideRootScale" null null))
      (bind _attachtransform_2 (`/Game/Blueprints/EndlessCells/BP_ObstaclePosition2.GetAttachpointTransform` _returnvalue_2))
      (set `self.NextSpawnPoint` _attachtransform_2))
    (:`Out 2`
      (bind _returnvalue_3 (`|SpawnActorFromClass` "/Game/Blueprints/EndlessCells/BP_ObstaclePosition3.BP_ObstaclePosition3_C" (`self.NextSpawnPoint`) "Undefined" "OverrideRootScale" null null))
      (bind _attachtransform_3 (`/Game/Blueprints/EndlessCells/BP_ObstaclePosition3.GetAttachpointTransform` _returnvalue_3))
      (set `self.NextSpawnPoint` _attachtransform_3))
    (:`Out 3`
      (bind _returnvalue_4 (`|SpawnActorFromClass` "/Game/Blueprints/EndlessCells/BP_ObstaclePosition4.BP_ObstaclePosition4_C" (`self.NextSpawnPoint`) "Undefined" "OverrideRootScale" null null))
      (bind _attachtransform_4 (`/Game/Blueprints/EndlessCells/BP_ObstaclePosition4.GetAttachpointTransform` _returnvalue_4))
      (set `self.NextSpawnPoint` _attachtransform_4))
    (:`Out 4`
      (bind _returnvalue_5 (`|SpawnActorFromClass` "/Game/Blueprints/EndlessCells/BP_ObstaclePosition5.BP_ObstaclePosition5_C" (`self.NextSpawnPoint`) "Undefined" "OverrideRootScale" null null))
      (bind _attachtransform_5 (`/Game/Blueprints/EndlessCells/BP_ObstaclePosition5.GetAttachpointTransform` _returnvalue_5))
      (set `self.NextSpawnPoint` _attachtransform_5))
    (:`Out 5`
      (bind _returnvalue_6 (`|SpawnActorFromClass` "/Game/Blueprints/EndlessCells/BP_ObstaclePosition3.BP_ObstaclePosition3_C" (`self.NextSpawnPoint`) "Undefined" "OverrideRootScale" null null))
      (bind _attachtransform_6 (`/Game/Blueprints/EndlessCells/BP_ObstaclePosition3.GetAttachpointTransform` _returnvalue_6))
      (set `self.NextSpawnPoint` _attachtransform_6))
    (:`Out 6`
      (bind _returnvalue_7 (`|SpawnActorFromClass` "/Game/Blueprints/EndlessCells/BP_ObstaclePosition1.BP_ObstaclePosition1_C" (`self.NextSpawnPoint`) "Undefined" "OverrideRootScale" null null))
      (bind _attachtransform_7 (`/Game/Blueprints/EndlessCells/BP_ObstaclePosition1.GetAttachpointTransform` _returnvalue_7))
      (set `self.NextSpawnPoint` _attachtransform_7))
    (:`Out 7`
      (bind _returnvalue_8 (`|SpawnActorFromClass` "/Game/Blueprints/EndlessCells/BP_ObstaclePosition2.BP_ObstaclePosition2_C" (`self.NextSpawnPoint`) "Undefined" "OverrideRootScale" null null))
      (bind _attachtransform_8 (`/Game/Blueprints/EndlessCells/BP_ObstaclePosition2.GetAttachpointTransform` _returnvalue_8))
      (set `self.NextSpawnPoint` _attachtransform_8))
    (:`Out 8`
      (bind _returnvalue_9 (`|SpawnActorFromClass` "/Game/Blueprints/EndlessCells/BP_ObstaclePosition3.BP_ObstaclePosition3_C" (`self.NextSpawnPoint`) "Undefined" "OverrideRootScale" null null))
      (bind _attachtransform_9 (`/Game/Blueprints/EndlessCells/BP_ObstaclePosition3.GetAttachpointTransform` _returnvalue_9))
      (set `self.NextSpawnPoint` _attachtransform_9))))

(fn `AddSpawner`
  (if (< (`self.CellSpawned`) 10)
    (bind _returnvalue (`|SpawnActorFromClass` "/Game/Blueprints/EndlessCells/BP_SpawnerCellNormal.BP_SpawnerCellNormal_C" (`self.NextSpawnPoint`) "Undefined" "OverrideRootScale" null null))
    (bind _attachtransform (`/Game/Blueprints/EndlessCells/BP_SpawnerCellNormal.GetAttachpointTransform` _returnvalue))
    (set `self.NextSpawnPoint` _attachtransform)
    (elif (< (`self.CellSpawned`) 20)
      (bind _returnvalue_2 (`|SpawnActorFromClass` "/Game/Blueprints/EndlessCells/BP_SpawnerCellMedium.BP_SpawnerCellMedium_C" (`self.NextSpawnPoint`) "Undefined" "OverrideRootScale" null null))
      (bind _attachtransform_2 (`/Game/Blueprints/EndlessCells/BP_SpawnerCellMedium.GetAttachpointTransform` _returnvalue_2))
      (set `self.NextSpawnPoint` _attachtransform_2)
      (elif (< (`self.CellSpawned`) 30)
        (bind _returnvalue_3 (`|SpawnActorFromClass` "/Game/Blueprints/EndlessCells/BP_SpawnerCellHard.BP_SpawnerCellHard_C" (`self.NextSpawnPoint`) "Undefined" "OverrideRootScale" null null))
        (bind _attachtransform_3 (`/Game/Blueprints/EndlessCells/BP_SpawnerCellHard.GetAttachpointTransform` _returnvalue_3))
        (set `self.NextSpawnPoint` _attachtransform_3)))))

(fn `EnemyKilled`
  (`/Engine/EditorBlueprintResources/StandardMacros.IncrementInt` (`self.i_EnemyKilled`)
    (:`  `
      (`self.UpdateEnemyCount` -1))))

(fn `GameOver`
  (bind _returnvalue (`GameplayStatics.GetPlayerController` 0))
  (bind _i_score (`self.i_Score`))
  (bind _bp_savegame (`self.BP_SaveGame`))
  ;[1 1 1] Shows GameOver HUD
  (bind _returnvalue_2 (`|CreateWidget` "/Game/Blueprints/GUI/BPW_GameOver.BPW_GameOver_C"))
  (`UserWidget.AddToViewport` _returnvalue_2 0)
  (set `PlayerController.bShowMouseCursor` true _returnvalue)
  (`WidgetBlueprintLibrary.SetInputMode_UIOnlyEx` _returnvalue _returnvalue_2)
  (set `self.i_HighScore` (`self.i_Score`))
  ;[1 1 1] Saves the highscore
  (bind _returnvalue_3 (`GameplayStatics.DoesSaveGameExist` "HighscoreData"))
  (if _returnvalue_3
    (bind _returnvalue_4 (`GameplayStatics.LoadGameFromSlot` "HighscoreData"))
    (bind _output_get (set `self.BP_SaveGame` _returnvalue_4))
    (bind _asbp_save_game (cast `/Game/Blueprints/GeneralGameBP/BP_SaveGame` _output_get))
    (if (> _i_score (`/Game/Blueprints/GeneralGameBP/BP_SaveGame.Highscore` _asbp_save_game))
      (set `/Game/Blueprints/GeneralGameBP/BP_SaveGame.Highscore` _i_score _asbp_save_game)
      (`GameplayStatics.SaveGameToSlot` _bp_savegame "HighscoreData"))
    (else
      (bind _returnvalue_5 (`GameplayStatics.CreateSaveGameObject` "/Game/Blueprints/GeneralGameBP/BP_SaveGame.BP_SaveGame_C"))
      (bind _output_get_2 (set `self.BP_SaveGame` _returnvalue_5))
      (bind _asbp_save_game_2 (cast `/Game/Blueprints/GeneralGameBP/BP_SaveGame` _output_get_2))
      (set `/Game/Blueprints/GeneralGameBP/BP_SaveGame.Highscore` _i_score _asbp_save_game_2)
      (`GameplayStatics.SaveGameToSlot` _bp_savegame "HighscoreData"))))

(fn `LoadScore`)

(fn `ResetMultiplier`
  (return))

(fn `SaveScore`)

(fn `SetMultiplier`
  (params (Value :type Integer))
  (set `self.i_Score` (* Value (`self.i_Score`))))

(fn `SetScore`
  (params (Value :type Integer))
  (bind _output_get (set `self.i_Score` (+ Value (`self.i_Score`))))
  (if (>= _output_get (`self.i_HighScore`))
    (set `self.i_HighScore` (`self.i_Score`))
    (else
      (set `self.i_HighScore` (`self.i_HighScore`)))))

(fn `UpdateEnemyCount`
  (params (Value :type Integer))
  (set `self.i_NormalEnemyCount` (+ (`self.i_NormalEnemyCount`) Value)))

(fn `UserConstructionScript`)