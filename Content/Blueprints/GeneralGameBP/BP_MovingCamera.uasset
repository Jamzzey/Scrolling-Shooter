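; BP_MovingCamera is an actor meant to scroll upward during play, but its movement logic is currently disconnected and never runs.
; On BeginPlay it caches references to BP_GameMode and BP_Player.
; The orphaned logic checks CameraMoving and that no boss has spawned, then plays the MoveCamera timeline to raise the actor along Z by CameraMovementSpeed on each update.
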(event `self.ReceiveBeginPlay`
  (bind _asbp_game_mode (cast `/Game/Blueprints/BP_GameMode` (`GameplayStatics.GetGameMode`)))
  (set `self.BP_GameMode` _asbp_game_mode)
  (bind _asbp_player (cast `/Game/Blueprints/Player/BP_Player` (`GameplayStatics.GetPlayerPawn` 0)))
  (set `self.BP_Player` _asbp_player))

(fn `UserConstructionScript`)