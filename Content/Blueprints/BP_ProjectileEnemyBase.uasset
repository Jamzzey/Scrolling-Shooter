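; BP_ProjectileEnemyBase is an enemy projectile actor, apparently a base class, that damages the player on contact.
; The construction script creates a dynamic glow material and applies the configurable scale and speed to the mesh and projectile movement.
; BeginPlay tints the material with the configured color.
; When the projectile overlaps BP_Player, it applies its damage, prints a debug message and destroys itself, ignoring other actors.
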(event `self.ReceiveBeginPlay`
  (`MaterialInstanceDynamic.SetVectorParameterValue` (`self.m_ProjectileMaterial`) "Color" (`self.c_ProjectileColor`)))

(event `self.Projectile.OnComponentBeginOverlap`
  (params (OverlappedComponent :type "PrimitiveComponent Object Reference") (OtherActor :type "Actor Object Reference") (OtherComp :type "PrimitiveComponent Object Reference") (OtherBodyIndex :type Integer) (bFromSweep :type Boolean) (SweepResult :type "HitResult Structure (by ref)"))
  (bind _asbp_player (cast `/Game/Blueprints/BP_Player` OtherActor))
  (`KismetSystemLibrary.PrintString` "Player has been damaged" true true (struct :`G` 0.66 :`B` 1.0 :`A` 1.0) 5.0)
  (`GameplayStatics.ApplyDamage` _asbp_player (`self.f_Damage`))
  (`self.K2_DestroyActor`))

(fn `UserConstructionScript`
  (bind _projectilemovement (`self.ProjectileMovement`))
  (bind _returnvalue (`PrimitiveComponent.CreateDynamicMaterialInstance` (`self.Projectile`) 0 "/Game/Assets/Materials/Glow/M_Glow_Projectile.M_Glow_Projectile" "None"))
  (set `self.m_ProjectileMaterial` _returnvalue)
  (`SceneComponent.SetWorldScale3D` (`self.Projectile`) (`self.v_Scale`))
  (bind _output_get (set `ProjectileMovementComponent.MaxSpeed` (`self.f_Speed`) _projectilemovement))
  (set `ProjectileMovementComponent.InitialSpeed` _output_get _projectilemovement))