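; BP_EnemyPathDouble is an enemy built to glide between random points while firing two projectiles at once.
; BeginPlay caches three component locations and picks a random target index.
; A timeline update holds the lerp movement, delayed re-targeting and delay-gated twin BP_Projectile spawns.
; Nothing starts that timeline: the pawn-sensing event only casts to BP_Player, so movement and shooting never run.
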(event `self.PawnSensing.OnSeePawn`
  (params (Pawn :type "Pawn Object Reference"))
  (cast `/Game/Blueprints/BP_Player` Pawn))

(event `self.ReceiveBeginPlay`
  ;[1 1 1] Creating the array of locations the enemy will move to
  (set `self.MoveToLocationPoints` (`|MakeArray` (`SceneComponent.K2_GetComponentLocation` (`self.MoveLocation1`)) (`SceneComponent.K2_GetComponentLocation` (`self.MoveLocation2`)) (`SceneComponent.K2_GetComponentLocation` (`self.MoveLocation3`))))
  (`self.GetRandomLocation`))

(fn `GetRandomLocation`
  (set `self.CurrentLocationPoint` (`KismetMathLibrary.RandomInteger` (`KismetArrayLibrary.Array_Length` (`self.MoveToLocationPoints`)))))

(fn `UserConstructionScript`)