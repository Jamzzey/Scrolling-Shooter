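; Dual-shot enemy variant that fires pairs of green default enemy projectiles from two scene-component muzzles.
; Once the parent's spawn animation enables firing, a random roll each Tick starts a delayed shot.
; A second delay then destroys the most recently spawned pair.
; The construction script applies a configurable scale to the mesh.
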(event `self.ReceiveBeginPlay`
  (`parent.ReceiveBeginPlay`))

(event `self.ReceiveTick`
  (params (DeltaSeconds :type "Float (single-precision)"))
  (`parent.ReceiveTick` DeltaSeconds)
  (if (`self.b_FiringEnabled`)
    (if (< (`KismetMathLibrary.RandomFloat`) (`self.FireChance`))
      (`KismetSystemLibrary.Delay` (`self.f_FiringDelay`))
      (bind _returnvalue (`|SpawnActorFromClass` "/Game/Blueprints/EnemyProjectiles/BP_ProjectileEnemyDefault.BP_ProjectileEnemyDefault_C" (`SceneComponent.K2_GetComponentToWorld` (`self.Scene2`)) "Undefined" "OverrideRootScale" null (struct :`R` 0.020136 :`G` 1.0) null))
      (bind _returnvalue_2 (`|SpawnActorFromClass` "/Game/Blueprints/EnemyProjectiles/BP_ProjectileEnemyDefault.BP_ProjectileEnemyDefault_C" (`SceneComponent.K2_GetComponentToWorld` (`self.Scene3`)) "Undefined" "OverrideRootScale" null (struct :`R` 0.020136 :`G` 1.0) null))
      (`KismetSystemLibrary.Delay` 2.0)
      (`self.K2_DestroyActor` _returnvalue)
      (`self.K2_DestroyActor` _returnvalue_2))))

(fn `UserConstructionScript`
  (`parent.UserConstructionScript`)
  (`SceneComponent.SetWorldScale3D` (`self.StaticMesh`) (`self.Scale`)))