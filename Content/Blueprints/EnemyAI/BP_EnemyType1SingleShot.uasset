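; Enemy type 1, a child enemy Blueprint that drifts at a constant velocity and fires single red projectiles at random.
; Tick moves the actor without sweep and, once the parent's spawn animation enables firing, rolls against FireChance to spawn a BP_ProjectileEnemyDefault at the Scene transform.
; Delays on the Tick chain postpone each shot briefly and later destroy the spawned projectile.
; Construction applies the Scale variable to the static mesh.
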(event `self.ReceiveBeginPlay`
  (`parent.ReceiveBeginPlay`))

(event `self.ReceiveTick`
  (params (DeltaSeconds :type "Float (single-precision)"))
  (`parent.ReceiveTick` DeltaSeconds)
  (`self.K2_AddActorWorldOffset` (`self.Constant Move Speed`))
  (if (`self.b_FiringEnabled`)
    (if (< (`KismetMathLibrary.RandomFloat`) (`self.FireChance`))
      (`KismetSystemLibrary.Delay` 0.1)
      (bind _returnvalue (`|SpawnActorFromClass` "/Game/Blueprints/EnemyProjectiles/BP_ProjectileEnemyDefault.BP_ProjectileEnemyDefault_C" (`SceneComponent.K2_GetComponentToWorld` (`self.Scene`)) "Undefined" "OverrideRootScale" null (struct :`R` 1.0 :`G` 0.055598) null))
      (`KismetSystemLibrary.Delay` 2.0)
      (`/Engine/EditorBlueprintResources/StandardMacros.IsValid` _returnvalue
        (:`Is Valid`
          (`self.K2_DestroyActor` _returnvalue))))))

(fn `UserConstructionScript`
  (`parent.UserConstructionScript`)
  (`SceneComponent.SetWorldScale3D` (`self.StaticMesh`) (`self.Scale`)))