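; BP_Boss2 is a boss enemy whose death triggers the level two win.
; BeginPlay caches BP_GameMode and turns on its destroy-all-enemies flag to cull other enemies.
; Damage shakes the camera and lowers clamped health; at zero it explodes, destroys itself, updates game mode flags (including LevelOneBossDead), clears widgets and calls LevelTwoGameWin.
; The timeline-driven projectile volley from many spawn points is disconnected, and overlap events are empty.
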(event `self.Cylinder4.OnComponentBeginOverlap`
  (params (OverlappedComponent :type "PrimitiveComponent Object Reference") (OtherActor :type "Actor Object Reference") (OtherComp :type "PrimitiveComponent Object Reference") (OtherBodyIndex :type Integer) (bFromSweep :type Boolean) (SweepResult :type "HitResult Structure (by ref)")))

(event `self.Cylinder3.OnComponentBeginOverlap`
  (params (OverlappedComponent :type "PrimitiveComponent Object Reference") (OtherActor :type "Actor Object Reference") (OtherComp :type "PrimitiveComponent Object Reference") (OtherBodyIndex :type Integer) (bFromSweep :type Boolean) (SweepResult :type "HitResult Structure (by ref)")))

(event `self.Cylinder2.OnComponentBeginOverlap`
  (params (OverlappedComponent :type "PrimitiveComponent Object Reference") (OtherActor :type "Actor Object Reference") (OtherComp :type "PrimitiveComponent Object Reference") (OtherBodyIndex :type Integer) (bFromSweep :type Boolean) (SweepResult :type "HitResult Structure (by ref)")))

(event `self.Cylinder1.OnComponentBeginOverlap`
  (params (OverlappedComponent :type "PrimitiveComponent Object Reference") (OtherActor :type "Actor Object Reference") (OtherComp :type "PrimitiveComponent Object Reference") (OtherBodyIndex :type Integer) (bFromSweep :type Boolean) (SweepResult :type "HitResult Structure (by ref)")))

(event `self.Cube.OnComponentBeginOverlap`
  (params (OverlappedComponent :type "PrimitiveComponent Object Reference") (OtherActor :type "Actor Object Reference") (OtherComp :type "PrimitiveComponent Object Reference") (OtherBodyIndex :type Integer) (bFromSweep :type Boolean) (SweepResult :type "HitResult Structure (by ref)")))

(event `self.ReceiveAnyDamage`
  (params (Damage :type "Float (single-precision)") (DamageType :type "DamageType Object Reference") (InstigatedBy :type "Controller Object Reference") (DamageCauser :type "Actor Object Reference"))
  (bind _returnvalue (`self.K2_GetActorLocation`))
  (bind _bp_gamemode (`self.BP_GameMode`))
  ;[1 1 1] Healthpoints Logic
  (`GameplayStatics.PlayWorldCameraShake` "/Game/Blueprints/GeneralGameBP/BP_CameraShake.BP_CameraShake_C" (`self.K2_GetActorLocation`) 0.0 500.0)
  (set `self.CurrentHealth` (`KismetMathLibrary.FClamp` (- (`self.CurrentHealth`) Damage) 0.0 (`self.MaximumHealth`)))
  (if (<= (`self.CurrentHealth`) 0.0)
    (`GameplayStatics.SpawnEmitterAtLocation` "/Game/Assets/Particles/P_Pixel_Explosion_Player.P_Pixel_Explosion_Player" _returnvalue)
    (`GameplayStatics.PlaySoundAtLocation` "/Game/Assets/Audio/Explosion_Clip.Explosion_Clip" _returnvalue (struct) 1.0 1.0 0.0 null null null)
    (set `/Game/Blueprints/BP_GameMode.DestroyAllEnemiesTrigger` false _bp_gamemode)
    (`self.K2_DestroyActor`)
    (set `/Game/Blueprints/BP_GameMode.LevelOneBossDead` true _bp_gamemode)
    (set `/Game/Blueprints/BP_GameMode.BossSpawned` false _bp_gamemode)
    (`WidgetLayoutLibrary.RemoveAllWidgets`)
    (`/Game/Blueprints/BP_GameMode.LevelTwoGameWin` _bp_gamemode)))

(event `self.ReceiveBeginPlay`
  ;[1 1 1] Set references then set Enemy culling to on
  (bind _asbp_game_mode (cast `/Game/Blueprints/BP_GameMode` (`GameplayStatics.GetGameMode`)))
  (bind _output_get (set `self.BP_GameMode` _asbp_game_mode))
  (set `/Game/Blueprints/BP_GameMode.DestroyAllEnemiesTrigger` true _output_get))

(fn `UserConstructionScript`)