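; BP_EnemyBase is an enemy base that sweeps along X at random speed, reversing on non-projectile hits.
; BeginPlay registers with BP_GameMode and enables movement, firing and damage; its spawn Timeline never runs.
; Lethal damage may drop one of four random pickups, plays explosion feedback, and updates game-mode kills and score multiplier.
; Overlapping the player deals damage and destroys the enemy directly, skipping that death logic.
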(event `self.ReceiveHit`
  (params (MyComp :type "PrimitiveComponent Object Reference") (Other :type "Actor Object Reference") (OtherComp :type "PrimitiveComponent Object Reference") (bSelfMoved :type Boolean) (HitLocation :type "Vector Structure") (HitNormal :type "Vector Structure") (NormalImpulse :type "Vector Structure") (Hit :type "HitResult Structure (by ref)"))
  ;[1 1 1] Reverse Direction Upon Hitting a Wall
  (cast `/Game/Blueprints/PlayerProjectiles/BP_ProjectilePlayerBase` Other
    (:`CastFailed`
      (set `self.b_MovementDirection` (not (`self.b_MovementDirection`))))))

(event `self.ReceiveTick`
  (params (DeltaSeconds :type "Float (single-precision)"))
  ;[1 1 1] Continous Movement after spawning
  (if (`self.b_MovementEnabled`)
    (`self.K2_SetActorLocation` (+ (`self.K2_GetActorLocation`) (* (`KismetMathLibrary.MakeVector` (* (`self.f_MovementSpeed`) (`KismetMathLibrary.SelectFloat` 1.0 -1.0 (`self.b_MovementDirection`)))) DeltaSeconds)) true)))

(event `self.ReceiveBeginPlay`
  (bind _v_spawnlocation (`self.v_SpawnLocation`))
  ;[1 1 1] Get reference to the variables and set them
  (bind _asbp_game_mode (cast `/Game/Blueprints/BP_GameMode` (`GameplayStatics.GetGameMode`)))
  (bind _output_get (set `self.BP_GameMode` _asbp_game_mode))
  (`/Game/Blueprints/BP_GameMode.CheckEnemyCount` _output_get 0)
  (set `self.b_MovementDirection` (`KismetMathLibrary.RandomBool`))
  (set `self.f_MovementSpeed` (`KismetMathLibrary.RandomFloatInRange` (`self.MininumSpeed`) (`self.MaximumSpeed`)))
  (set `self.v_SpawnLocation` (`self.K2_GetActorLocation`))
  ;[1 1 1] Spawn Animation
  (set `self.b_MovementEnabled` true)
  (set `self.b_FiringEnabled` true)
  (set `self.b_TakeDamageEnabled` true)
  (`self.K2_SetActorLocation` (`KismetMathLibrary.VLerp` _v_spawnlocation (- _v_spawnlocation (10.0 0.0 120.0)) 1.0)))

(event `self.StaticMesh.OnComponentBeginOverlap`
  (params (OverlappedComponent :type "PrimitiveComponent Object Reference") (OtherActor :type "Actor Object Reference") (OtherComp :type "PrimitiveComponent Object Reference") (OtherBodyIndex :type Integer) (bFromSweep :type Boolean) (SweepResult :type "HitResult Structure (by ref)"))
  ;[1 1 1] Collision with Player, set to destroy the enemy for now
  (bind _asbp_player (cast `/Game/Blueprints/BP_Player` OtherActor))
  (`GameplayStatics.ApplyDamage` _asbp_player (`self.Collision Damage to Player`))
  (`self.K2_DestroyActor`))

(event `self.ReceiveAnyDamage`
  (params (Damage :type "Float (single-precision)") (DamageType :type "DamageType Object Reference") (InstigatedBy :type "Controller Object Reference") (DamageCauser :type "Actor Object Reference"))
  (bind _returnvalue (`self.K2_GetActorLocation`))
  (bind _returnvalue_2 (`self.K2_GetActorLocation`))
  ;[1 1 1] Health Calculation
  (if (`self.b_TakeDamageEnabled`)
    (set `self.CurrentHealth` (`KismetMathLibrary.FClamp` (- (`self.CurrentHealth`) Damage) 0.0 (`self.MaximumHealth`)))
    (if (<= (`self.CurrentHealth`) 0.0)
      ;[1 1 1] Drop Rate of Pickup
      (if (< (`KismetMathLibrary.RandomFloat`) (`self.Pickup Drop Chance`))
        (`|MultiGate` true
          (:`Out 0`
            ;[1 1 1] Set the Power Ups here
            (`|SpawnActorFromClass` "/Game/Blueprints/WeaponCollectible/BP_PickUp_NewWeaponMode.BP_PickUp_NewWeaponMode_C" (`KismetMathLibrary.MakeTransform` _returnvalue (struct) (4.0 4.0 4.0)) "Undefined" "OverrideRootScale" null null))
          (:`Out 1`
            (`|SpawnActorFromClass` "/Game/Blueprints/PickUps/BP_PickUp_DefaultFireRate.BP_PickUp_DefaultFireRate_C" (`KismetMathLibrary.MakeTransform` _returnvalue (struct) (4.0 4.0 4.0)) "Undefined" "OverrideRootScale" null null))
          (:`Out 2`
            (`|SpawnActorFromClass` "/Game/Blueprints/PickUps/BP_PickUp_CloneShips.BP_PickUp_CloneShips_C" (`KismetMathLibrary.MakeTransform` _returnvalue (struct) (4.0 4.0 4.0)) "Undefined" "OverrideRootScale" null null))
          (:`Out 3`
            (`|SpawnActorFromClass` "/Game/Blueprints/PickUps/BP_PickUp_AddShield.BP_PickUp_AddShield_C" (`KismetMathLibrary.MakeTransform` _returnvalue (struct) (4.0 4.0 4.0)) "Undefined" "OverrideRootScale" null null))))
      ;[1 1 1] Player Feedback, FX, Shake and Sound
      (`GameplayStatics.SpawnEmitterAtLocation` "/Game/Assets/Particles/P_Pixel_Explosion_Player.P_Pixel_Explosion_Player" _returnvalue_2)
      (`GameplayStatics.PlayWorldCameraShake` "/Game/Blueprints/BP_CameraShake.BP_CameraShake_C" _returnvalue_2 0.0 500.0)
      (`GameplayStatics.PlaySoundAtLocation` "/Game/Assets/Audio/Explosion.Explosion" _returnvalue_2 (struct) 1.0 1.0 0.0 null null null)
      (`self.EnemyKilled`)
      (`self.K2_DestroyActor`))))

(fn `EnemyKilled`
  (bind _bp_gamemode (`self.BP_GameMode`))
  (`/Game/Blueprints/BP_GameMode.EnemyKilled` _bp_gamemode)
  (if true
    (`/Game/Blueprints/BP_GameMode.SetScore` _bp_gamemode 0)
    (set `/Game/Blueprints/BP_GameMode.i_Multiplier` (+ (`self.MultiplierValue`) 2) _bp_gamemode)
    (`/Game/Blueprints/BP_GameMode.Multiply` _bp_gamemode)))

(fn `UserConstructionScript`)