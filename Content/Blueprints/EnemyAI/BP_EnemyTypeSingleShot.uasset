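; Enemy Blueprint that fires single red projectiles at random once the parent's spawn animation enables firing.
; Each Tick rolls against FireChance, then after a short Delay spawns a BP_ProjectileEnemyDefault at the Scene component's transform.
; A second Delay precedes destroying the spawned projectile, with both latent nodes running directly off Tick.
; The construction script applies Scale to the static mesh after calling the parent's.
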(event `self.ReceiveBeginPlay`
  (`parent.ReceiveBeginPlay`))

(event `self.ReceiveTick`
  (params (DeltaSeconds :type "Float (single-precision)"))
  (`parent.ReceiveTick` DeltaSeconds)
  (if (`self.b_FiringEnabled`)
    (if (< (`KismetMathLibrary.RandomFloat`) (`self.FireChance`))
      (`KismetSystemLibrary.Delay` 0.1)
      (bind _returnvalue (`|SpawnActorFromClass` "/Game/Blueprints/EnemyProjectiles/BP_ProjectileEnemyDefault.BP_ProjectileEnemyDefault_C" (`SceneComponent.K2_GetComponentToWorld` (`self.Scene`)) "Undefined" "OverrideRootScale" null (struct :`R` 1.0 :`G` 0.030353) null))
      (`KismetSystemLibrary.Delay` 2.0)
      (`self.K2_DestroyActor` _returnvalue))))

(fn `UserConstructionScript`
  (`parent.UserConstructionScript`)
  (`SceneComponent.SetWorldScale3D` (`self.StaticMesh`) (`self.Scale`)))