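; BP_ProjectilePlayerBase is, by its name, a base projectile for the player, with configurable color, scale and speed.
; The construction script creates a dynamic glow material instance on the Projectile component, sets that component's world scale, and feeds the speed variable into ProjectileMovement as both max and initial speed.
; BeginPlay then applies the projectile color to the material's Color parameter.
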(event `self.ReceiveBeginPlay`
  (`MaterialInstanceDynamic.SetVectorParameterValue` (`self.m_ProjectileMaterial`) "Color" (`self.c_ProjectileColor`)))

(fn `UserConstructionScript`
  (bind _projectilemovement (`self.ProjectileMovement`))
  (bind _returnvalue (`PrimitiveComponent.CreateDynamicMaterialInstance` (`self.Projectile`) 0 "/Game/Assets/Materials/Glow/M_Glow_Projectile.M_Glow_Projectile" "None"))
  (set `self.m_ProjectileMaterial` _returnvalue)
  (`SceneComponent.SetWorldScale3D` (`self.Projectile`) (`self.v_Scale`))
  (bind _output_get (set `ProjectileMovementComponent.MaxSpeed` (`self.f_Speed`) _projectilemovement))
  (set `ProjectileMovementComponent.InitialSpeed` _output_get _projectilemovement))