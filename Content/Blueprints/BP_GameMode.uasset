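; Game mode that builds a randomized level from cells and obstacles, tracks score and enemy counts, and shows the HUD and game-over screen.
; BeginPlay alternates cell and obstacle spawns, each picked by random MultiGate and chained through the previous piece's attach-point transform.
; Score functions update the high score, apply multipliers and count kills.
; LoadScore and SaveScore are empty stubs, and the Medium, Hard and Boss cell functions duplicate AddCell.
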(event `self.ReceiveBeginPlay`
  ;[1 1 1] HUD
  (`WidgetBlueprintLibrary.SetInputMode_GameOnly` (`GameplayStatics.GetPlayerController` 0))
  (`self.LoadScore`)
  (`self.SetScore` 0)
  (bind _returnvalue (`|CreateWidget` "/Game/Blueprints/GUI/BPW_HUD.BPW_HUD_C"))
  (bind _output_get (set `self.BPW_Hud` _returnvalue))
  (`UserWidget.AddToViewport` _output_get 0)
  ;[1 1 1] Spawn Level
  (for _ (range 2)
    (`self.AddCell`)
    (`self.AddObstacle`)))

(event `self.ReceiveEndPlay`
  (params (EndPlayReason :type "EEndPlayReason Enum" :default "Destroyed"))
  (`self.SaveScore`))

(event `Multiply`
  (set `self.i_Score` (* (`self.i_Score`) (`self.i_Multiplier`)))
  (`KismetSystemLibrary.Delay` 5.0)
  (set `self.i_Multiplier` (- (`self.i_Multiplier`) 1)))

(event `CheckEnemyCount`
  (params (Value :type Integer)))

(fn `AddArray`
  (returns (Output :type "/Game/Blueprints/EndlessCells/BP_CellOne Object Reference"))
  (locals (NewLocalVar_0 :type "/Game/Blueprints/EndlessCells/BP_CellOne Object Reference"))
  (bind _outactors (`GameplayStatics.GetAllActorsOfClass` "/Game/Blueprints/EndlessCells/BP_CellOne.BP_CellOne_C"))
  (return (`|GetArrayItem` _outactors (`KismetMathLibrary.RandomInteger` (`KismetArrayLibrary.Array_Length` _outactors)))))

(fn `AddBossCell`
  (`|MultiGate` true
    (:`Out 0`
      (bind _returnvalue (`|SpawnActorFromClass` "/Game/Blueprints/EndlessCells/BP_CellOne.BP_CellOne_C" (`self.NextSpawnPoint`) "Undefined" "OverrideRootScale" null null))
      (bind _attachtransform (`/Game/Blueprints/EndlessCells/BP_CellOne.GetAttachpointTransform` _returnvalue))
      (set `self.NextSpawnPoint` _attachtransform))
    (:`Out 1`
      (bind _returnvalue_2 (`|SpawnActorFromClass` "/Game/Blueprints/EndlessCells/BP_CellTwo.BP_CellTwo_C" (`self.NextSpawnPoint`) "Undefined" "OverrideRootScale" null null))
      (bind _attachtransform_2 (`/Game/Blueprints/EndlessCells/BP_CellOne.GetAttachpointTransform` _returnvalue_2))
      (set `self.NextSpawnPoint` _attachtransform_2))
    (:`Out 2`
      (bind _returnvalue_3 (`|SpawnActorFromClass` "/Game/Blueprints/EndlessCells/BP_CellThree.BP_CellThree_C" (`self.NextSpawnPoint`) "Undefined" "OverrideRootScale" null null))
      (bind _attachtransform_3 (`/Game/Blueprints/EndlessCells/BP_CellOne.GetAttachpointTransform` _returnvalue_3))
      (set `self.NextSpawnPoint` _attachtransform_3))))

(fn `AddCell`
  (`|MultiGate` true
    (:`Out 0`
      (bind _returnvalue (`|SpawnActorFromClass` "/Game/Blueprints/EndlessCells/BP_CellOne.BP_CellOne_C" (`self.NextSpawnPoint`) "Undefined" "OverrideRootScale" null null))
      (bind _attachtransform (`/Game/Blueprints/EndlessCells/BP_CellOne.GetAttachpointTransform` _returnvalue))
      (set `self.NextSpawnPoint` _attachtransform))
    (:`Out 1`
      (bind _returnvalue_2 (`|SpawnActorFromClass` "/Game/Blueprints/EndlessCells/BP_CellTwo.BP_CellTwo_C" (`self.NextSpawnPoint`) "Undefined" "OverrideRootScale" null null))
      (bind _attachtransform_2 (`/Game/Blueprints/EndlessCells/BP_CellOne.GetAttachpointTransform` _returnvalue_2))
      (set `self.NextSpawnPoint` _attachtransform_2))
    (:`Out 2`
      (bind _returnvalue_3 (`|SpawnActorFromClass` "/Game/Blueprints/EndlessCells/BP_CellThree.BP_CellThree_C" (`self.NextSpawnPoint`) "Undefined" "OverrideRootScale" null null))
      (bind _attachtransform_3 (`/Game/Blueprints/EndlessCells/BP_CellOne.GetAttachpointTransform` _returnvalue_3))
      (set `self.NextSpawnPoint` _attachtransform_3))))

(fn `AddHardCell`
  (`|MultiGate` true
    (:`Out 0`
      (bind _returnvalue (`|SpawnActorFromClass` "/Game/Blueprints/EndlessCells/BP_CellOne.BP_CellOne_C" (`self.NextSpawnPoint`) "Undefined" "OverrideRootScale" null null))
      (bind _attachtransform (`/Game/Blueprints/EndlessCells/BP_CellOne.GetAttachpointTransform` _returnvalue))
      (set `self.NextSpawnPoint` _attachtransform))
    (:`Out 1`
      (bind _returnvalue_2 (`|SpawnActorFromClass` "/Game/Blueprints/EndlessCells/BP_CellTwo.BP_CellTwo_C" (`self.NextSpawnPoint`) "Undefined" "OverrideRootScale" null null))
      (bind _attachtransform_2 (`/Game/Blueprints/EndlessCells/BP_CellOne.GetAttachpointTransform` _returnvalue_2))
      (set `self.NextSpawnPoint` _attachtransform_2))
    (:`Out 2`
      (bind _returnvalue_3 (`|SpawnActorFromClass` "/Game/Blueprints/EndlessCells/BP_CellThree.BP_CellThree_C" (`self.NextSpawnPoint`) "Undefined" "OverrideRootScale" null null))
      (bind _attachtransform_3 (`/Game/Blueprints/EndlessCells/BP_CellOne.GetAttachpointTransform` _returnvalue_3))
      (set `self.NextSpawnPoint` _attachtransform_3))))

(fn `AddMediumCell`
  (`|MultiGate` true
    (:`Out 0`
      (bind _returnvalue (`|SpawnActorFromClass` "/Game/Blueprints/EndlessCells/BP_CellOne.BP_CellOne_C" (`self.NextSpawnPoint`) "Undefined" "OverrideRootScale" null null))
      (bind _attachtransform (`/Game/Blueprints/EndlessCells/BP_CellOne.GetAttachpointTransform` _returnvalue))
      (set `self.NextSpawnPoint` _attachtransform))
    (:`Out 1`
      (bind _returnvalue_2 (`|SpawnActorFromClass` "/Game/Blueprints/EndlessCells/BP_CellTwo.BP_CellTwo_C" (`self.NextSpawnPoint`) "Undefined" "OverrideRootScale" null null))
      (bind _attachtransform_2 (`/Game/Blueprints/EndlessCells/BP_CellOne.GetAttachpointTransform` _returnvalue_2))
      (set `self.NextSpawnPoint` _attachtransform_2))
    (:`Out 2`
      (bind _returnvalue_3 (`|SpawnActorFromClass` "/Game/Blueprints/EndlessCells/BP_CellThree.BP_CellThree_C" (`self.NextSpawnPoint`) "Undefined" "OverrideRootScale" null null))
      (bind _attachtransform_3 (`/Game/Blueprints/EndlessCells/BP_CellOne.GetAttachpointTransform` _returnvalue_3))
      (set `self.NextSpawnPoint` _attachtransform_3))))

(fn `AddObstacle`
  (`|MultiGate` true
    (:`Out 0`
      (bind _returnvalue (`|SpawnActorFromClass` "/Game/Blueprints/EndlessCells/BP_ObstaclePosition1.BP_ObstaclePosition1_C" (`self.NextSpawnPoint`) "Undefined" "OverrideRootScale" null null))
      (bind _attachtransform (`/Game/Blueprints/EndlessCells/BP_ObstaclePosition1.GetAttachpointTransform` _returnvalue))
      (set `self.NextSpawnPoint` _attachtransform))
    (:`Out 1`
      (bind _returnvalue_2 (`|SpawnActorFromClass` "/Game/Blueprints/EndlessCells/BP_ObstaclePosition2.BP_ObstaclePosition2_C" (`self.NextSpawnPoint`) "Undefined" "OverrideRootScale" null null))
      (bind _attachtransform_2 (`/Game/Blueprints/EndlessCells/BP_ObstaclePosition2.GetAttachpointTransform` _returnvalue_2))
      (set `self.NextSpawnPoint` _attachtransform_2))
    (:`Out 2`
      (bind _returnvalue_3 (`|SpawnActorFromClass` "/Game/Blueprints/EndlessCells/BP_ObstaclePosition3.BP_ObstaclePosition3_C" (`self.NextSpawnPoint`) "Undefined" "OverrideRootScale" null null))
      (bind _attachtransform_3 (`/Game/Blueprints/EndlessCells/BP_ObstaclePosition3.GetAttachpointTransform` _returnvalue_3))
      (set `self.NextSpawnPoint` _attachtransform_3))))

(fn `EnemyKilled`
  (`/Engine/EditorBlueprintResources/StandardMacros.IncrementInt` (`self.i_EnemyKilled`)
    (:`  `
      (`self.UpdateEnemyCount` -1))))

(fn `GameOver`
  (bind _returnvalue (`GameplayStatics.GetPlayerController` 0))
  (bind _returnvalue_2 (`|CreateWidget` "/Game/Blueprints/GUI/BPW_GameOver.BPW_GameOver_C"))
  (`UserWidget.AddToViewport` _returnvalue_2 0)
  (set `PlayerController.bShowMouseCursor` true _returnvalue)
  (`WidgetBlueprintLibrary.SetInputMode_UIOnlyEx` _returnvalue _returnvalue_2))

(fn `LoadScore`)

(fn `ResetMultiplier`
  (return))

(fn `SaveScore`)

(fn `SetMultiplier`
  (params (Value :type Integer))
  (set `self.i_Score` (* Value (`self.i_Score`))))

(fn `SetScore`
  (params (Value :type Integer))
  (bind _output_get (set `self.i_Score` (+ Value (`self.i_Score`))))
  (if (>= _output_get (`self.i_HighScore`))
    (set `self.i_HighScore` (`self.i_Score`))
    (else
      (set `self.i_HighScore` (`self.i_HighScore`)))))

(fn `UpdateEnemyCount`
  (params (Value :type Integer))
  (set `self.i_EnemyCount` (+ (`self.i_EnemyCount`) Value)))

(fn `UserConstructionScript`)