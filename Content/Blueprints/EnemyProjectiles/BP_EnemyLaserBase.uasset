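; Laser enemy that slides side to side along X, fires at random, and damages the player on overlap.
; BeginPlay calls the GameMode's enemy-count check, randomizes direction and speed, then runs a spawn Timeline that enables movement and firing.
; Tick does swept movement, reversed by hits from anything except player projectiles, and rolls to fire a laser, pausing movement briefly.
; At zero health it may drop a pickup, then explodes with shake and sound.
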(event `self.ReceiveHit`
  (params (MyComp :type "PrimitiveComponent Object Reference") (Other :type "Actor Object Reference") (OtherComp :type "PrimitiveComponent Object Reference") (bSelfMoved :type Boolean) (HitLocation :type "Vector Structure") (HitNormal :type "Vector Structure") (NormalImpulse :type "Vector Structure") (Hit :type "HitResult Structure (by ref)"))
  (cast `/Game/Blueprints/PlayerProjectiles/BP_ProjectilePlayerBase` Other
    (:`CastFailed`
      (set `self.b_MovementDirection` (not (`self.b_MovementDirection`))))))

(event `self.ReceiveTick`
  (params (DeltaSeconds :type "Float (single-precision)"))
  (if (`self.b_MovementEnabledLaser`)
    (`self.K2_SetActorLocation` (+ (`self.K2_GetActorLocation`) (* (`KismetMathLibrary.MakeVector` (* (`self.f_MovementSpeed`) (`KismetMathLibrary.SelectFloat` 1.0 -1.0 (`self.b_MovementDirection`)))) DeltaSeconds)) true)
    (if (`self.b_FiringEnabled`)
      (if (< (`KismetMathLibrary.RandomFloat`) (`self.FireChance`))
        (set `self.b_MovementEnabledLaser` false)
        (`|SpawnActorFromClass` "/Game/Blueprints/EnemyProjectiles/BP_ProjectileEnemyLaser.BP_ProjectileEnemyLaser_C" (`SceneComponent.K2_GetComponentToWorld` (`self.Scene`)) "Undefined" "OverrideRootScale" null (struct :`R` 1.0 :`B` 0.951129) null)
        (`KismetSystemLibrary.Delay` 2.0)
        (set `self.b_MovementEnabledLaser` true)))))

(event `self.ReceiveBeginPlay`
  (bind _v_spawnlocation (`self.v_SpawnLocation`))
  ;[1 1 1] Set References to variables
  (bind _asbp_game_mode (cast `/Game/Blueprints/BP_GameMode` (`GameplayStatics.GetGameMode`)))
  (bind _output_get (set `self.BP_GameMode` _asbp_game_mode))
  (`/Game/Blueprints/BP_GameMode.CheckEnemyCount` _output_get 0)
  (set `self.b_MovementDirection` (`KismetMathLibrary.RandomBool`))
  (set `self.f_MovementSpeed` (`KismetMathLibrary.RandomFloatInRange` (`self.f_MininumSpeed`) (`self.f_MaximumSpeed`)))
  (set `self.v_SpawnLocation` (`self.K2_GetActorLocation`))
  ;[1 1 1] Spawn Animation
  (bind (_direction _entryspeed) (`Timeline|Spawn`)
    (:`Update`
      (`self.K2_SetActorLocation` (`KismetMathLibrary.VLerp` _v_spawnlocation (- _v_spawnlocation (10.0 0.0 120.0)) _entryspeed)))
    (:`Finished`
      (set `self.b_MovementEnabledLaser` true)
      (set `self.b_FiringEnabled` true))))

(event `self.StaticMesh.OnComponentBeginOverlap`
  (params (OverlappedComponent :type "PrimitiveComponent Object Reference") (OtherActor :type "Actor Object Reference") (OtherComp :type "PrimitiveComponent Object Reference") (OtherBodyIndex :type Integer) (bFromSweep :type Boolean) (SweepResult :type "HitResult Structure (by ref)"))
  ;[1 1 1] Collision with Player, set to destroy the enemy for now
  (bind _asbp_player (cast `/Game/Blueprints/BP_Player` OtherActor))
  (`KismetSystemLibrary.PrintString` "Player has been damaged!" true true (struct :`G` 0.66 :`B` 1.0 :`A` 1.0) 5.0)
  (`GameplayStatics.ApplyDamage` _asbp_player (`self.Damage`)))

(event `self.ReceiveAnyDamage`
  (params (Damage :type "Float (single-precision)") (DamageType :type "DamageType Object Reference") (InstigatedBy :type "Controller Object Reference") (DamageCauser :type "Actor Object Reference"))
  (bind _returnvalue (`self.K2_GetActorLocation`))
  (bind _returnvalue_2 (`self.GetTransform`))
  ;[1 1 1] Health Calculation
  (set `self.f_Health` (`KismetMathLibrary.FClamp` (- (`self.f_Health`) Damage) 0.0 (`self.f_MaximumHealth`)))
  (if (<= (`self.f_Health`) 0.0)
    (if (< (`KismetMathLibrary.RandomFloat`) (`self.Drop Chance`))
      (if (< (`KismetMathLibrary.RandomFloat`) (`self.Drop Chance`))
        ;[1 1 1] Set the Power Ups here
        (`|SpawnActorFromClass` "/Game/Blueprints/WeaponCollectible/BP_PickUp_NewWeaponMode.BP_PickUp_NewWeaponMode_C" _returnvalue_2 "Undefined" "OverrideRootScale" null null)
        (elif (< (`KismetMathLibrary.RandomFloat`) (`self.Drop Chance`))
          (`|SpawnActorFromClass` "/Game/Blueprints/PickUps/BP_PickUp_DefaultFireRate.BP_PickUp_DefaultFireRate_C" _returnvalue_2 "Undefined" "OverrideRootScale" null null)
          (else
            (`|SpawnActorFromClass` "/Game/Blueprints/PickUps/BP_PickUp_DefaultFireRate.BP_PickUp_DefaultFireRate_C" _returnvalue_2 "Undefined" "OverrideRootScale" null null)))))
    ;[1 1 1] Player Feedback, FX, Shake and Sound
    (`GameplayStatics.SpawnEmitterAtLocation` "/Game/Assets/Particles/P_Pixel_Explosion_Player.P_Pixel_Explosion_Player" _returnvalue)
    (`GameplayStatics.PlayWorldCameraShake` "/Game/Blueprints/BP_CameraShake.BP_CameraShake_C" _returnvalue 0.0 500.0)
    (`GameplayStatics.PlaySoundAtLocation` "/Game/Assets/Audio/Explosion.Explosion" _returnvalue (struct) 1.0 1.0 0.0 null null null)
    (`KismetSystemLibrary.PrintString` "Enemy is dead!")
    (`self.K2_DestroyActor`)))

(fn `UserConstructionScript`)