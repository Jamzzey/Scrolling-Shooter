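; BP_EnemyLaser is an enemy that starts at the first of four location markers and fires a laser when it sees the player.
; Pawn sensing starts a delayed sequence that spawns BP_Laser at LaserSpawn, later destroys it, then calls MoveToLocation.
; MoveToLocation only picks a random point index.
; The Timeline meant to lerp the actor toward that point and re-enter the firing branch is never triggered.
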(event `self.ReceiveBeginPlay`
  ;[1 1 1] creating array
  (set `self.LocationPoints` (`|MakeArray` (`SceneComponent.K2_GetComponentLocation` (`self.Location1`)) (`SceneComponent.K2_GetComponentLocation` (`self.Location2`)) (`SceneComponent.K2_GetComponentLocation` (`self.Location3`)) (`SceneComponent.K2_GetComponentLocation` (`self.Location4`))))
  (`self.K2_SetActorLocation` (`SceneComponent.K2_GetComponentLocation` (`self.Location1`))))

(event `self.PawnSensing.OnSeePawn`
  (params (Pawn :type "Pawn Object Reference"))
  ;[1 1 1] if the enemy is in the right location shoot laser
  (cast `/Game/Blueprints/BP_Player` Pawn)
  (set `self.InLocation` true)
  (if (`self.InLocation`)
    (`KismetSystemLibrary.Delay` 6.0)
    (bind _returnvalue (`|SpawnActorFromClass` "/Game/Blueprints/BP_Laser.BP_Laser_C" (`SceneComponent.K2_GetComponentToWorld` (`self.LaserSpawn`)) "Undefined" "OverrideRootScale" null null))
    (`KismetSystemLibrary.Delay` 4.0)
    (set `self.InLocation` false)
    (`self.K2_DestroyActor` _returnvalue)
    (`KismetSystemLibrary.Delay` 6.0)
    (`self.MoveToLocation`)
    (else
      ;[1 1 1] move to another location
      (`KismetSystemLibrary.Delay` 6.0)
      (`self.MoveToLocation`))))

(fn `MoveToLocation`
  (set `self.CurrentLocationPoint` (`KismetMathLibrary.RandomInteger` (`KismetArrayLibrary.Array_Length` (`self.LocationPoints`)))))

(fn `UserConstructionScript`)