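; BP_Boss is a boss Blueprint built to shoot BP_BossProjectile2 in continuous volleys.
; A timeline update spawns one projectile at each of four ShootProjectileLocation components.
; The ShootProjectile flag gates each volley, clearing after the spawns and resetting after ShootDelay.
; Nothing starts the timeline, so the firing logic never runs as wired, and the construction script is empty.
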(fn `UserConstructionScript`)