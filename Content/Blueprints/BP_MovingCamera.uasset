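; BP_MovingCamera is an actor intended as a scrolling camera that moves along world Z until a boss spawns.
; On BeginPlay it casts the game mode to BP_GameMode and caches it for the BossSpawned check.
; Its MoveCamera timeline would add CameraMovementSpeed to Z each update while CameraMoving is set, but that chain is unconnected, so this graph never moves the actor.
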(event `self.ReceiveBeginPlay`
  (bind _asbp_game_mode (cast `/Game/Blueprints/BP_GameMode` (`GameplayStatics.GetGameMode`)))
  (set `self.BP_GameMode` _asbp_game_mode))

(fn `UserConstructionScript`)